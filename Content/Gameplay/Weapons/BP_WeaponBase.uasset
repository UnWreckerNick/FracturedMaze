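; Base weapon Blueprint with ammo-limited hitscan firing.
; WeaponFire decrements AmmoCount when positive, then calls PerformLineTrace and PlayFireEffect, which spawns a muzzle flash and, only if that flash is valid, plays the fire sound.
; The Visibility trace adds Range to a zero-rotation forward vector instead of scaling it, ignoring aim, and only prints whether it hit.
; WeaponReload and the event graph are empty stubs.
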(fn `PerformLineTrace`
  (bind _outhit (`KismetSystemLibrary.LineTraceSingle` (`self.MuzzleLocation`) (+ (`self.MuzzleLocation`) (`KismetMathLibrary.GetForwardVector` (struct)) (`self.Range`)) "TraceTypeQuery1"))
  (`KismetSystemLibrary.PrintString` (`KismetStringLibrary.Conv_BoolToString` (`GameplayStatics.BreakHitResult` _outhit)))
  (return))

(fn `PlayFireEffect`
  (`/Engine/EditorBlueprintResources/StandardMacros.IsValid` (`self.MuzzleFlash`)
    (:`Is Valid`
      (`GameplayStatics.SpawnEmitterAtLocation` (`self.MuzzleFlash`) (`self.MuzzleLocation`) (struct) (0.3 0.3 0.3))
      (`/Engine/EditorBlueprintResources/StandardMacros.IsValid` (`self.FireSound`)
        (:`Is Valid`
          (`GameplayStatics.PlaySoundAtLocation` (`self.FireSound`) (`self.MuzzleLocation`) (struct) 1.0 1.0 0.0 null null null null)
          (return))))))

(fn `UserConstructionScript`)

(fn `WeaponFire`
  (if (> (`self.AmmoCount`) 0)
    (`/Engine/EditorBlueprintResources/StandardMacros.DecrementInt` (`self.AmmoCount`)
      (:`  `
        (`self.PerformLineTrace`)
        (`self.PlayFireEffect`)
        (return)))))

(fn `WeaponReload`)